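; Player tank pawn that creates its HUD, switches between default, machine and high-velocity projectiles, and has a speed boost with an overheat penalty.
; Each ammo slot caches the projectile's cost and fire rate from class defaults and updates the hotbar.
; Held fire loops through a fire-rate delay, spending ammo and playing the matching HUD reload animation.
; Tick-driven delay macros raise and cool heat, temporarily slowing the tank at maximum.
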(event EventBeginPlay
  (Utilities|FlowControl|Sequence
    (:then_0
      (bind _returnvalue (UserInterface|CreateWidget "/Game/Blueprints/Widgets/HUD/HUD.HUD_C"))
      (bind _output_get (Variables|Default|SetHUD _returnvalue))
      (UserInterface|Viewport|AddtoViewport _output_get 0)
      (Variables|Default|SetHUDAmmoBar (Variables|/Game/Blueprints/Widgets/HUD/HUD.HUD_C|GetAmmoBar _output_get)))
    (:then_1
      ;[1 1 1] Get Default Projectile Ammo Cost
      (bind _output_get_2 (Variables|Default|SetProjectileClass "/Game/Blueprints/InGame_BPs/Projectiles/BP_DefaultProjectile.BP_DefaultProjectile_C"))
      (Utilities|FlowControl|Sequence
        (:then_0
          (Variables|Default|SetcurrentAmmoCost (.AmmoCost (Utilities|GetClassDefaults _output_get_2))))
        (:then_1
          (Variables|Default|SetCurrentFireRate (.FireRate (Utilities|GetClassDefaults _output_get_2)))
          (Default|SelectHotBarSlotOne (Variables|Default|GetHUDAmmoBar)))))))

(event EventTick
  (params (DeltaSeconds :type Float%20%28single-precision%29))
  (Utilities|FlowControl|Sequence
    (:then_0
      ;[0 0.000251 0.01562 1 60] Overheat Mechanic
      ;;[1 1 1] Begin Overheat if Speed up is activated
      (if (== (Variables|Default|GetCurrentSpeed) (Variables|Default|GetSpeedUpSpeed))
        (Utilities|IncreasingOverheat)
        ;;[1 1 1] Tank Overheated... Slowed down for set delay time
        (if (>= (Variables|Default|GetOverheat) (Variables|Default|GetMaxOverheat))
          (Utilities|TankOverheated)
          ;;[1 1 1] Resets Tank back to Default Speed
          (Variables|Default|SetbOverheated false)
          (Variables|Default|SetCurrentSpeed (Variables|Default|GetNormalSpeed)))
        (else
          ;;[1 1 1] If Overheat = True Tank is cooling down. Show this in UI somehow?
          (if (Variables|Default|GetbOverheated)
            (Development|PrintString "Cooling Down...")
            (Utilities|DecreasingOverheat)
            (else
              ;;[1 1 1] Makes sure overheat doesn't go below 0. If not zero, decrease overheat my 2 every 0.2secs
              (if (<= (Variables|Default|GetOverheat) 0.0)
                (Variables|Default|SetOverheat 0.0)
                (else
                  (Utilities|DecreasingOverheat))))))))))

(event Input|ActionEvents|InputActionSpeedUp
  (params (Key :type Key%20Structure :default "None"))
  (bind _boverheated (Variables|Default|GetbOverheated))
  ;[1 1 1 1 24] Speed Up Ability (See Overheat Mechanic for more Details)
  (:Pressed
    (if (not _boverheated)
      (Variables|Default|SetCurrentSpeed (Variables|Default|GetSpeedUpSpeed))))
  (:Released
    (if (not _boverheated)
      (Variables|Default|SetCurrentSpeed (Variables|Default|GetNormalSpeed)))))

(event Input|ActionEvents|InputActionAmmoTwo
  (params (Key :type Key%20Structure :default "None"))
  ;[1 1 1] Get Machine Projectile Ammo Cost
  (:Pressed
    (bind _output_get (Variables|Default|SetProjectileClass "/Game/Blueprints/InGame_BPs/Projectiles/BP_MachineProjectile.BP_MachineProjectile_C"))
    (Utilities|FlowControl|Sequence
      (:then_0
        (Variables|Default|SetcurrentAmmoCost (.AmmoCost (Utilities|GetClassDefaults _output_get))))
      (:then_1
        (Variables|Default|SetCurrentFireRate (.FireRate (Utilities|GetClassDefaults _output_get)))
        (Default|SelectHotBarSlotTwo (Variables|Default|GetHUDAmmoBar))))))

(event Input|ActionEvents|InputActionAmmoThree
  (params (Key :type Key%20Structure :default "None"))
  ;[1 1 1] Get High Velocity Projectile Ammo Cost
  (:Pressed
    (bind _output_get (Variables|Default|SetProjectileClass "/Game/Blueprints/InGame_BPs/Projectiles/BP_HighVelocityProjectile.BP_HighVelocityProjectile_C"))
    (Utilities|FlowControl|Sequence
      (:then_0
        (Variables|Default|SetcurrentAmmoCost (.AmmoCost (Utilities|GetClassDefaults _output_get))))
      (:then_1
        (Variables|Default|SetCurrentFireRate (.FireRate (Utilities|GetClassDefaults _output_get)))
        (Default|SelectHotBarSlotThree (Variables|Default|GetHUDAmmoBar))))))

(event Input|ActionEvents|InputActionAmmoOne
  (params (Key :type Key%20Structure :default "None"))
  ;[1 1 1] Get Default Projectile Ammo Cost
  (:Pressed
    (bind _output_get (Variables|Default|SetProjectileClass "/Game/Blueprints/InGame_BPs/Projectiles/BP_DefaultProjectile.BP_DefaultProjectile_C"))
    (Utilities|FlowControl|Sequence
      (:then_0
        (Variables|Default|SetcurrentAmmoCost (.AmmoCost (Utilities|GetClassDefaults _output_get))))
      (:then_1
        (Variables|Default|SetCurrentFireRate (.FireRate (Utilities|GetClassDefaults _output_get)))
        (Default|SelectHotBarSlotOne (Variables|Default|GetHUDAmmoBar))))))

(event Input|ActionEvents|InputActionFire
  (params (Key :type Key%20Structure :default "None"))
  ;[1 1 1] Fire Conditions (If there is enough ammo left, then fire. Delay by FireRate).
  (:Pressed
    (Variables|Default|SetbIsTriggerPressed true)
    (if (Variables|Default|GetbIsTriggerPressed) :!label _label
      (if (Variables|Default|GetbCanFire)
        (Variables|Default|SetbCanFire false)
        (if (> (Variables|Default|GetcurrentAmmoCost) (Variables|Default|GetAmmoRemaining))
          (Variables|Default|SetbCanFire true)
          (Development|PrintString "Not Enough Ammo")
          (else
            (Class|BasePawn|Fire)
            (Variables|Default|SetAmmoRemaining (- (Variables|Default|GetAmmoRemaining) (Variables|Default|GetcurrentAmmoCost)))
            (CallFunction|PlayReloadAnim)
            (Utilities|FlowControl|Delay (Variables|Default|GetCurrentFireRate))
            (Variables|Default|SetbCanFire true)
            (goto _label))))))
  (:Released
    (Variables|Default|SetbIsTriggerPressed false)))

(fn ConstructionScript)

(fn PlayReloadAnim
  (bind _hud (Variables|Default|GetHUD))
  (bind _hud_2 (Variables|Default|GetHUD))
  (bind _hud_3 (Variables|Default|GetHUD))
  (bind _reloadturret (Variables|/Game/Blueprints/Widgets/HUD/HUD.HUD_C|GetReloadTurret _hud))
  (bind _reloadturret_2 (Variables|/Game/Blueprints/Widgets/HUD/HUD.HUD_C|GetReloadTurret _hud_2))
  (bind _reloadturret_3 (Variables|/Game/Blueprints/Widgets/HUD/HUD.HUD_C|GetReloadTurret _hud_3))
  (bind _output_get (Variables|Default|SetCurrent%20Ammo%20Type (Variables|/Game/Blueprints/Widgets/HUD/HUDComponents/ProjectileBar.ProjectileBar_C|GetCurrentAmmoType (Variables|/Game/Blueprints/Widgets/HUD/HUD.HUD_C|GetAmmoBar (Variables|Default|GetHUD)))))
  (if (== _output_get 1)
    (UserInterface|Animation|PlayAnimation _reloadturret_3 (Variables|/Game/Blueprints/Widgets/HUD/HUDComponents/ReloadTurret.ReloadTurret_C|GetDefaultReload _reloadturret_3) 0.0 1 "Forward" 1.0 false)
    (elif (== _output_get 2)
      (UserInterface|Animation|PlayAnimation _reloadturret (Variables|/Game/Blueprints/Widgets/HUD/HUDComponents/ReloadTurret.ReloadTurret_C|GetAutoReload _reloadturret) 0.0 1 "Forward" 1.0 false)
      (elif (== _output_get 3)
        (UserInterface|Animation|PlayAnimation _reloadturret_2 (Variables|/Game/Blueprints/Widgets/HUD/HUDComponents/ReloadTurret.ReloadTurret_C|GetSniperReload _reloadturret_2) 0.0 1 "Forward" 1.0 false)))))