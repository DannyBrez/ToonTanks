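; Machine turret pawn Blueprint that drives the turret's health bar widget.
; Each Tick it passes the health component's current-to-max ratio, clamped between 0 and 1, to the TurretHealthBar widget.
; It then caches the player's DefaultTank pawn and shows the bar only while that tank overlaps the VisableRange component.
; The graphs contain no aiming or firing logic.
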(event EventBeginPlay)

(event Collision|EventActorBeginOverlap
  (params (OtherActor :type Actor%20Object%20Reference)))

(event EventTick
  (params (DeltaSeconds :type Float%20%28single-precision%29))
  (bind _healthbarwidget (Variables|Default|GetHealthBarWidget))
  (bind _asturret_health_bar (Utilities|Casting|CastToTurretHealthBar (UserInterface|GetUserWidgetObject (Variables|Default|GetHealthBarWidget))))
  (CallFunction|SetHealthonWidget _asturret_health_bar)
  (bind _asdefault_tank (Utilities|Casting|CastToDefaultTank (Game|Player|GetPlayerPawn 0)))
  (Variables|Default|SetPlayerRef _asdefault_tank)
  (if (Collision|IsOverlappingActor (Variables|Default|GetVisableRange) (Variables|Default|GetPlayerRef) :!class /Script/Engine.PrimitiveComponent)
    (Rendering|SetVisibility _healthbarwidget true false)
    (else
      (Rendering|SetVisibility _healthbarwidget false false))))

(fn ConstructionScript)

(fn SetHealthonWidget
  (params (self2 :type Turret%20Health%20Bar%20Object%20Reference))
  (bind _healthcomponents (Variables|Default|GetHealthComponents))
  (Variables|/Game/Blueprints/Widgets/TurretHealthBar.TurretHealthBar_C|SetRemainingHealthWidget self2 (Math|Float|Clamp(Float) (/ (Variables|/Script/ToonTanks.HealthComponent|GetHealth _healthcomponents) (Variables|/Script/ToonTanks.HealthComponent|GetMaxHealth _healthcomponents)))))